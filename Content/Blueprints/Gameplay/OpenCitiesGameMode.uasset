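; Game mode that runs an in-game clock and calendar and simulates population change across City actors.
; Tick advances a scaled 24-hour clock and pushes time and date to the game state for client clocks.
; Each day rollover adds births through fractional accumulators, then splits each city's emigrants among others using normalized population-ratio scores.
; City actors are scaled by population at start and after births.
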(event `self.ReceiveBeginPlay`
  ;[1 1 1] Initialize populations and sizes of cities
  (`|ExecutionSequence`
    (:`then_0`
      (bind _outactors (`GameplayStatics.GetAllActorsOfClass` "/Game/Blueprints/City.City_C"))
      (for _array_element _outactors
        (bind _output_get (set `self.City` _array_element))
        (`self.Resize Cities` _output_get
          (:`NewParam`
            (bind _asmy_game_state (cast `/Game/Blueprints/MyGameState` (`GameplayStatics.GetGameState`)))
            (set `self.GameStateRef` _asmy_game_state)))))
    (:`then_1`
      (set `self.Clockwork` (+ (`KismetMathLibrary.Conv_IntToDouble` (`self.Hours`)) (/ (`KismetMathLibrary.Conv_IntToDouble` (`self.Minutes`)) 60.0) (/ (`KismetMathLibrary.Conv_IntToDouble` (`self.Seconds`)) 3600.0)))
      (set `/Game/Blueprints/MyGameState.GameDate` (`|MakeArray` (`self.Day`) (`self.Month`) (`self.Year`)) (`self.GameStateRef`)))))

(event `self.ReceiveTick`
  (params (DeltaSeconds :type "Float (single-precision)"))
  (bind (_clockwork _daytick) (`self.SetClockwork` DeltaSeconds))
  ;[1 1 1] Clockwork
  (set `self.Clockwork` _clockwork)
  (bind _output_get (set `self.Day Tick` _daytick))
  (if (== _output_get 1)
    (`self.CalculateCityProcesses`) ; Moving populations
  )
  (`self.Clock`)
  (`self.Calendar`))

(event `CalculateCityProcesses`
  ;[1 1 1] For Each City Calculate Stuff
  (bind _outactors (`GameplayStatics.GetAllActorsOfClass` "/Game/Blueprints/City.City_C"))
  (for _array_element _outactors
    (bind _output_get (set `self.ActiveCity` _array_element))
    (`|ExecutionSequence`
      (:`then_0`
        ;[1 1 1] Births
        (`self.Calculate Births For a City` _output_get))
      (:`then_1`
        ;[1 1 1] Calculate Probs for the cities that people will move
        (`self.ClearArrays` ; Clears Arrays that will contain moving scores
          (:`NewParam2`
            (bind _outactors_2 (`GameplayStatics.GetAllActorsOfClass` "/Game/Blueprints/City.City_C"))
            (bind _output_get_2 (set `self.AllOtherCities` _outactors_2))
            (`KismetArrayLibrary.Array_RemoveItem` _output_get_2 _output_get) ; Remove current city
            (for _array_element_2 _output_get_2
              (bind _output_get_3 (set `self.CityToMove` _array_element_2))
              (`self.CalculatePopulationScore` _output_get _output_get_3))
            ;[1 1 1] Move Populations based on their respective emmigration rates and other factors
            (`self.AggregateScores`
              (:`NewParam2`
                (for (_array_element_3 _array_index) (`self.MovingScores`)
                  (`KismetArrayLibrary.Array_Set` (`self.MovingScores`) _array_index (`KismetMathLibrary.Conv_IntToDouble` (`KismetMathLibrary.Round` (* (/ _array_element_3 (`self.MovingScoresSum`)) (`KismetMathLibrary.Conv_IntToDouble` (`KismetMathLibrary.Round` (* (`/Game/Blueprints/City.DailyEmmigrationRate` _output_get) (`KismetMathLibrary.Conv_IntToDouble` (`/Game/Blueprints/City.Population` _output_get))))))))))
                (for (_array_element_4 _array_index_2) (`self.MovingScores`)
                  (`self.MovePopulations` (`self.ActiveCity`) (`KismetArrayLibrary.Array_Get` (`self.AllOtherCities`) _array_index_2) (`KismetMathLibrary.FTrunc` _array_element_4)))))))))))

(fn `Calendar`
  (bind _output_get (set `self.Day` (+ (`self.Day`) (`self.Day Tick`))))
  (if (> _output_get (`KismetMathLibrary.DaysInMonth` (`self.Year`) (`self.Month`)))
    (set `self.Day` 1)
    (set `self.Month` (+ (`self.Month`) 1)))
  (if (> (`self.Month`) 12)
    (set `self.Month` 1)
    (set `self.Year` (+ (`self.Year`) 1)))
  (set `/Game/Blueprints/MyGameState.GameDate` (`|MakeArray` (`self.Day`) (`self.Month`) (`self.Year`)) (`self.GameStateRef`)))

(fn `Clock`
  (bind _gamestateref (`self.GameStateRef`))
  (bind (_remainder _returnvalue) (`KismetMathLibrary.FMod` (* (`self.Clockwork`) 3600.0) 60.0))
  (bind (_remainder_2 _returnvalue_2) (`KismetMathLibrary.FMod` (`KismetMathLibrary.Conv_IntToDouble` _returnvalue) 60.0))
  (set `self.Seconds` (`KismetMathLibrary.FFloor` _remainder))
  (set `self.Minutes` (`KismetMathLibrary.FFloor` _remainder_2))
  (set `self.Hours` (`KismetMathLibrary.FFloor` (`KismetMathLibrary.FMod` (`KismetMathLibrary.Conv_IntToDouble` _returnvalue_2) 24.0)))
  (set `/Game/Blueprints/MyGameState.GameTime` (`|MakeArray` (`self.Seconds`) (`self.Minutes`) (`self.Hours`)) _gamestateref)
  (`/Game/Blueprints/MyGameState.UpdateClientClocks` _gamestateref))

(fn `PrintElementsofArray`
  (params (Array :type "Array of Float (double-precision)"))
  (bind _testvar (`self.TestVar`))
  (for _array_element Array
    (set `self.TestVar` (`KismetStringLibrary.Concat_StrStr` (`KismetStringLibrary.Conv_DoubleToString` _array_element) "," _testvar))
    (`KismetSystemLibrary.K2_PauseTimerHandle` (`self.Main World Timer`)))
  (`KismetSystemLibrary.PrintString` _testvar true true (struct :`G` 0.66 :`B` 1.0 :`A` 1.0) 165.0))

(fn `SetClockwork`
  (params (DeltaSeconds :type "Float (double-precision)"))
  (returns (Clockwork :type "Float (double-precision)") (DayTick :type Integer))
  (bind (_remainder _returnvalue) (`KismetMathLibrary.FMod` (+ (/ DeltaSeconds (`self.TimeUnit`)) (`self.Clockwork`)) 24.0))
  (return _remainder _returnvalue))

(fn `UserConstructionScript`)