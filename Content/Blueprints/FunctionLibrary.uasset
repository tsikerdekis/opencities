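; Function library of shared helpers for a city economy game with resources, taxes and trade deals.
; Resource lookup scans a city's sphere of influence, defaulting to the player's city, and Evil Corp prices come from a data table.
; Income helpers derive tax from population and basic income, sum accepted outgoing deals over capped days, and append daily or monthly records.
; Utilities lerp HUD positions in XY and pick random circle offsets using separate X and Y angles.
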(fn HUDLerpLocation
  (params (CurrentLocation :type Vector) (DestinationLocation :type Vector) (Speed :type Float%20%28single-precision%29))
  (bind _returnvalue (Math|Vector|Lerp(Vector) CurrentLocation DestinationLocation Speed))
  (return (Math|Vector|MakeVector (.x _returnvalue) (.y _returnvalue) (.Z (Math|Vector|BreakVector CurrentLocation)))))

(fn CheckifResourceExistsinCity
  (params (City :type City%20Object%20Reference) (Blueprint :type Actor%20Class%20Reference))
  (Utilities|IsValid City
    (:Is%20Valid
      (for _array_element (Collision|GetOverlappingActors (Variables|/Game/Blueprints/City.City_C|GetSphereOfInfluence City) "/Game/Blueprints/Resources/ResourceClass.ResourceClass_C" :!class /Script/Engine.PrimitiveComponent)
        (if (== (Utilities|GetClass _array_element) Blueprint)
          (return true _array_element))))
    (:Is%20Not%20Valid
      (bind _ascamera_pawn_controller (Utilities|Casting|CastToCameraPawnController (Game|GetPlayerController 0)))
      (for _array_element_2 (Collision|GetOverlappingActors (Variables|/Game/Blueprints/City.City_C|GetSphereOfInfluence (Variables|/Game/Blueprints/Characters/CameraPawn.CameraPawn_C|GetPlayerCity (Variables|/Game/Blueprints/Gameplay/CameraPawnController.CameraPawnController_C|GetCameraPawnRef _ascamera_pawn_controller))) "/Game/Blueprints/Resources/ResourceClass.ResourceClass_C" :!class /Script/Engine.PrimitiveComponent)
        (if (== Blueprint (Utilities|GetClass _array_element_2))
          (return true _array_element)))))
  (return false 0))

(fn GetCircleRandomCircumferencePoint
  (params (a :type Float%20%28single-precision%29) (b :type Float%20%28single-precision%29) (Radius :type Float%20%28single-precision%29))
  (bind _returnvalue (Math|Random|RandomFloatinRange 0.0 3.6e+02))
  (return (+ a (* (Math|Trig|Cos(Degrees) _returnvalue) Radius)) (+ b (* (Math|Trig|Sin(Degrees) _returnvalue) Radius))))

(fn GetEvilCorpPrice
  (params (Resource :type Resource%20Class%20Class%20Reference))
  (bind _outrownames (DataTable|GetDataTableRowNames "/Game/Blueprints/Gameplay/EvilCorpPriceTable.EvilCorpPriceTable"))
  (bind _array_element (Utilities|Array|ForEachLoopwithBreak _outrownames)
    (:LoopBody
      (bind _returnvalue (Utilities|GetDataTableRow "/Game/Blueprints/Gameplay/EvilCorpPriceTable.EvilCorpPriceTable" _array_element)
        (:then
          (if (== Resource (.blueprint _returnvalue))
            (return (.priceperunit _returnvalue))))))))

(fn CalculateTaxIncomeforCity
  (params (City :type City%20Object%20Reference))
  (Utilities|IsValid City
    (:Is%20Valid
      (bind _asmy_game_state (Utilities|Casting|CastToMyGameState (Game|GetGameState))
        (:then
          (return (Math|Float|Round (* (/ (Math|Conversions|ToFloat(Integer) (Variables|/Game/Blueprints/City.City_C|GetTaxRate City)) 1e+02) (Math|Conversions|ToFloat(Integer) (* (Variables|/Game/Blueprints/City.City_C|GetPopulation City) (Variables|/Game/Blueprints/Gameplay/MyGameState.MyGameState_C|GetBasicIncome _asmy_game_state)))))))
        (:CastFailed
          _)))
    (:Is%20Not%20Valid
      _))
  (return 0))

(fn CalculateTradeDealsIncomeforCity
  (params (City :type City%20Object%20Reference) (DaysInFutureLimit :type Integer))
  (LocalVariables|SetTotal 0)
  (bind _asmy_game_state (Utilities|Casting|CastToMyGameState (Game|GetGameState)))
  (for _array_element (Variables|/Game/Blueprints/Gameplay/MyGameState.MyGameState_C|GetTradeDeals _asmy_game_state)
    (if (and (and (== (.cityfrom _array_element) City) (!= (.days _array_element) 0)) (.accepted _array_element))
      (LocalVariables|SetTotal (+ (LocalVariables|GetTotal) (* (Math|Integer|Clamp(Integer) (.days _array_element) 0 DaysInFutureLimit) (* (.amount _array_element) (.price _array_element)))))))
  (return (LocalVariables|GetTotal)))

(fn AddtoCityRecords
  (params (City :type City%20Object%20Reference) (Daily :type Boolean) (Income :type Float%20%28single-precision%29) (Expense :type Float%20%28single-precision%29) (Type :type String))
  (if Daily
    (Utilities|Array|Add (Variables|/Game/Blueprints/City.City_C|GetDailyRecords City) (Utilities|Struct|MakeRecords Type Income Expense))
    (else
      (Utilities|Array|Add (Variables|/Game/Blueprints/City.City_C|GetMonthlyRecords City) (Utilities|Struct|MakeRecords Type Income Expense))))
  (return true))