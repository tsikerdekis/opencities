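; Lobby game mode Blueprint that simulates population growth and migration between City actors, scaling each actor by its population.
; CalculateCityProcesses first adds births per city, carrying fractional births in a BirthClock accumulator.
; It then scores other cities by relative population, standardizes and weights the scores, and splits daily emigrants proportionally among them.
; Cities resize on BeginPlay and after births, while migration only updates populations and prints each move.
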(event `self.ReceiveBeginPlay`
  ;[1 1 1] Initialize populations and sizes of cities
  (bind _outactors (`GameplayStatics.GetAllActorsOfClass` "/Game/Blueprints/City.City_C"))
  (for _array_element _outactors
    (bind _output_get (set `self.City` _array_element))
    (`self.Resize Cities` _output_get)))

(event `self.ReceiveTick`
  (params (DeltaSeconds :type "Float (single-precision)")))

(event `CalculateCityProcesses`
  ;[1 1 1] For Each City Calculate Stuff
  (bind _outactors (`GameplayStatics.GetAllActorsOfClass` "/Game/Blueprints/City.City_C"))
  (for _array_element _outactors
    (bind _output_get (set `self.ActiveCity` _array_element))
    (`|ExecutionSequence`
      (:`then_0`
        ;[1 1 1] Births
        (`self.Calculate Births For a City` _output_get))
      (:`then_1`
        ;[1 1 1] Calculate Probs for the cities that people will move
        (`self.ClearArrays` ; Clears Arrays that will contain moving scores
          (:`NewParam2`
            (bind _outactors_2 (`GameplayStatics.GetAllActorsOfClass` "/Game/Blueprints/City.City_C"))
            (bind _output_get_2 (set `self.AllOtherCities` _outactors_2))
            (`KismetArrayLibrary.Array_RemoveItem` _output_get_2 _output_get) ; Remove current city
            (for _array_element_2 _output_get_2
              (bind _output_get_3 (set `self.CityToMove` _array_element_2))
              (`self.CalculatePopulationScore` _output_get _output_get_3))
            ;[1 1 1] Move Populations based on their respective emmigration rates and other factors
            (`self.AggregateScores`
              (:`NewParam2`
                (for (_array_element_3 _array_index) (`self.MovingScores`)
                  (`KismetArrayLibrary.Array_Set` (`self.MovingScores`) _array_index (`KismetMathLibrary.Conv_IntToDouble` (`KismetMathLibrary.Round` (* (/ _array_element_3 (`self.MovingScoresSum`)) (`KismetMathLibrary.Conv_IntToDouble` (`KismetMathLibrary.Round` (* (`/Game/Blueprints/City.DailyEmmigrationRate` _output_get) (`KismetMathLibrary.Conv_IntToDouble` (`/Game/Blueprints/City.Population` _output_get))))))))))
                (for (_array_element_4 _array_index_2) (`self.MovingScores`)
                  (`self.MovePopulations` (`self.ActiveCity`) (`KismetArrayLibrary.Array_Get` (`self.AllOtherCities`) _array_index_2) (`KismetMathLibrary.FTrunc` _array_element_4)))))))))))

(fn `PrintElementsofArray`
  (params (Array :type "Array of Float (double-precision)"))
  (bind _testvar (`self.TestVar`))
  (for _array_element Array
    (set `self.TestVar` (`KismetStringLibrary.Concat_StrStr` (`KismetStringLibrary.Conv_DoubleToString` _array_element) "," _testvar))
    (`KismetSystemLibrary.K2_PauseTimerHandle` (`self.Main World Timer`)))
  (`KismetSystemLibrary.PrintString` _testvar true true (struct :`G` 0.66 :`B` 1.0 :`A` 1.0) 165.0))

(fn `UserConstructionScript`)