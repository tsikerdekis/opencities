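; Lobby player controller that drives an RTS-style camera pawn, creates the main HUD and passes clicked selectable actors to a HUD request.
; Axis input moves the pawn at a speed scaled by spring-arm zoom and a Shift boost, while screen-edge cursor checks add boosted local offsets.
; Holding Pan opens gates for mouse yaw and clamped pitch rotation and suspends movement; other inputs reset pitch or zoom the arm within limits.
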(event `self.ReceiveBeginPlay`
  (`|ExecutionSequence`
    (:`then_0`
      (`self.ReferenceCasts`))
    (:`then_1`
      (`WidgetBlueprintLibrary.SetInputMode_GameAndUIEx` self null true false)
      (`self.CreateHuds`)
      (`UserWidget.AddToViewport` (`self.MainHUDRef`) 0))
    (:`then_2`
      (set `self.bShowMouseCursor` true))))

(event `InputAction|Left Click`
  (params (Key :type "Key Structure" :default "AnyKey"))
  (bind (_bblockinghit _binitialoverlap _time _location _impactpoint _normal _impactnormal _physmat _hitactor) (`GameplayStatics.BreakHitResult` (`self.GetHitResultUnderCursorForObjects` (`self.SelectableObjectsENUM`))))
  (:`Pressed`
    (if (!= _hitactor null)
      (`self.HUDRequest` _hitactor))))

(event `InputAxis|MoveForward`
  (params (AxisValue :type "Float (single-precision)"))
  (bind _camerapawnref (`self.CameraPawnRef`))
  ;[1 1 1] Comment
  ;;[1 1 1] Movement X
  (if (not (`self.DisableCamNav`))
    (`self.K2_SetActorTransform` _camerapawnref (`self.MovementX` (`self.MovementSpeedCalculation`) (`self.FastMoveMultiplier`) AxisValue _camerapawnref) false false)))

(event `InputAxisKey|MouseX`
  (params (AxisValue :type "Float (single-precision)"))
  ;[1 1 1] Comment
  ;;[1 1 1] Pan X
  (`/Engine/EditorBlueprintResources/StandardMacros.Gate` true :!label _label
    (:`Exit`
      (`self.K2_SetActorRotation` (`self.CameraPawnRef`) (`KismetMathLibrary.MakeRotator` (.roll (`self.K2_GetActorRotation` (`self.CameraPawnRef`))) (.pitch (`self.K2_GetActorRotation` (`self.CameraPawnRef`))) (+ (.yaw (`self.K2_GetActorRotation` (`self.CameraPawnRef`))) (* (`self.PanSensitivity`) AxisValue))) false))))

(event `InputAction|Pan`
  (params (Key :type "Key Structure" :default "AnyKey"))
  ;[1 1 1] Comment
  ;;[1 1 1] Pan X
  (:`Pressed`
    (set `self.DisableCamNav` true)
    (goto _label :!via `Open`))
  (:`Released`
    (set `self.DisableCamNav` false)
    (goto _label :!via `Close`)))

(event `InputAxis|MoveRight`
  (params (AxisValue :type "Float (single-precision)"))
  (bind _camerapawnref (`self.CameraPawnRef`))
  ;[1 1 1] Comment
  ;;[1 1 1] Movement Y
  (if (not (`self.DisableCamNav`))
    (`self.K2_SetActorTransform` _camerapawnref (`KismetMathLibrary.MakeTransform` (`KismetMathLibrary.MakeVector` (.x (.location (`self.MovementY` AxisValue (`self.MovementSpeedCalculation`) (`self.FastMoveMultiplier`) _camerapawnref))) (.y (.location (`self.MovementY` AxisValue (`self.MovementSpeedCalculation`) (`self.FastMoveMultiplier`) _camerapawnref))) 100.0) (.rotation (`self.MovementY` AxisValue (`self.MovementSpeedCalculation`) (`self.FastMoveMultiplier`) _camerapawnref)) (.scale (`self.MovementY` AxisValue (`self.MovementSpeedCalculation`) (`self.FastMoveMultiplier`) _camerapawnref))) false false)))

(event `InputAxisKey|MouseY`
  (params (AxisValue :type "Float (single-precision)"))
  ;[1 1 1] Comment
  ;;[1 1 1] Pan Y
  (`/Engine/EditorBlueprintResources/StandardMacros.Gate` true :!label _label_2
    (:`Exit`
      (`self.K2_SetActorRotation` (`self.CameraPawnRef`) (`KismetMathLibrary.MakeRotator` (.roll (`self.K2_GetActorRotation` (`self.CameraPawnRef`))) (`KismetMathLibrary.FClamp` (+ (.pitch (`self.K2_GetActorRotation` (`self.CameraPawnRef`))) (* (`self.PanSensitivity`) AxisValue)) -15.0 45.0) (.yaw (`self.K2_GetActorRotation` (`self.CameraPawnRef`)))) false))))

(event `InputAction|Pan`
  (params (Key :type "Key Structure" :default "AnyKey"))
  ;[1 1 1] Comment
  ;;[1 1 1] Pan Y
  (:`Pressed`
    (set `self.DisableCamNav` true)
    (goto _label_2 :!via `Open`))
  (:`Released`
    (set `self.DisableCamNav` false)
    (goto _label_2 :!via `Close`)))

(event `Key|LeftShift`
  (params (Key :type "Key Structure" :default "AnyKey"))
  ;[1 1 1] Comment
  ;;[1 1 1] Move Multiplier
  (:`Pressed`
    (set `self.FastMoveMultiplier` 2.0))
  (:`Released`
    (set `self.FastMoveMultiplier` 1.0)))

(event `InputAction|PanReset`
  (params (Key :type "Key Structure" :default "AnyKey"))
  (bind _camerapawnref (`self.CameraPawnRef`))
  ;[1 1 1] Comment
  ;;[1 1 1] Pan Reset
  (:`Pressed`
    (`self.K2_SetActorRotation` _camerapawnref (`KismetMathLibrary.MakeRotator` (.roll (`self.K2_GetActorRotation` _camerapawnref)) 0.0 (.yaw (`self.K2_GetActorRotation` _camerapawnref))) false)))

(event `InputAction|ZoomIn`
  (params (Key :type "Key Structure" :default "AnyKey"))
  (bind _springarm (`/Game/Blueprints/Characters/CameraPawn.SpringArm` (`self.CameraPawnRef`)))
  ;[1 1 1] Comment
  ;;[1 1 1] Zoom In/Out
  (:`Pressed`
    (set `SpringArmComponent.TargetArmLength` (`KismetMathLibrary.FClamp` (- (`SpringArmComponent.TargetArmLength` _springarm) (`self.ZoomingSensitivity`)) 500.0 (`self.MaxArmDistance`)) _springarm)))

(event `InputAxisKey|MouseX`
  (params (AxisValue :type "Float (single-precision)"))
  ;[1 1 1] Comment
  ;;[1 1 1] Edge Movement
  (if (not (`self.DisableCamNav`))
    (bind (_deltayspeed _deltaxspeed) (`self.ScreenEdgeMovement` :!label _label_3))
    (`self.K2_AddActorLocalOffset` (`self.CameraPawnRef`) (`KismetMathLibrary.MakeVector` _deltaxspeed _deltayspeed) true false)))

(event `InputAxisKey|MouseY`
  (params (AxisValue :type "Float (single-precision)"))
  ;[1 1 1] Comment
  ;;[1 1 1] Edge Movement
  (if (not (`self.DisableCamNav`))
    (goto _label_3 :!via `MouseY`)))

(event `InputAction|ZoomOut`
  (params (Key :type "Key Structure" :default "AnyKey"))
  (bind _springarm (`/Game/Blueprints/Characters/CameraPawn.SpringArm` (`self.CameraPawnRef`)))
  ;[1 1 1] Comment
  ;;[1 1 1] Zoom In/Out
  (:`Pressed`
    (set `SpringArmComponent.TargetArmLength` (`KismetMathLibrary.FClamp` (+ (`self.ZoomingSensitivity`) (`SpringArmComponent.TargetArmLength` _springarm)) 500.0 (`self.MaxArmDistance`)) _springarm)))

(fn `MovementSpeedCalculation`
  (returns (MoveSensitivity :type "Float (double-precision)"))
  (return (`KismetMathLibrary.FClamp` (/ (`SpringArmComponent.TargetArmLength` (`/Game/Blueprints/Characters/CameraPawn.SpringArm` (`self.CameraPawnRef`))) 100.0) 5.0 20.0)))

(fn `Set Calendar`
  (params (Date :type "Array of Integer (by ref)"))
  (returns (Success :type Boolean))
  (return false))

(fn `Set Clock`
  (params (Time :type "Array of Integer (by ref)"))
  (returns (Success :type Boolean))
  (return false))

(fn `UserConstructionScript`)