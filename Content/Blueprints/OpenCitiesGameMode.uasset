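; Game mode that simulates city population growth, printing the world's day speed at start and scaling each City actor by normalized population.
; A Delay on Tick acts as the day clock, running births for every city with a fractional accumulator carried between days.
; It also builds max-standardized moving scores from population ratios between cities, but migration is unfinished: nothing applies them and CalculatePopulationScores is empty.
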(event `self.ReceiveBeginPlay`
  ;[1 1 1] Initialize populations and sizes of cities
  (`KismetSystemLibrary.PrintString` (`KismetStringLibrary.Concat_StrStr` "World speed is to 1 day every " (`KismetStringLibrary.Conv_IntToString` (`self.ClockSpeed`)) "seconds") true true (struct :`G` 0.66 :`B` 1.0 :`A` 1.0) 10.0)
  (bind _outactors (`GameplayStatics.GetAllActorsOfClass` "/Game/Blueprints/City.City_C"))
  (for _array_element _outactors
    (bind _output_get (set `self.City` _array_element))
    (`self.Resize Cities` _output_get)))

(event `self.ReceiveTick`
  (params (DeltaSeconds :type "Float (single-precision)"))
  ;[1 1 1] For each city estimate people that will move and to where
  (`KismetSystemLibrary.Delay` (`KismetMathLibrary.Conv_IntToDouble` (`self.ClockSpeed`)))
  (bind _outactors (`GameplayStatics.GetAllActorsOfClass` "/Game/Blueprints/City.City_C"))
  (for _array_element _outactors
    (bind _output_get (set `self.ActiveCity` _array_element))
    (`|ExecutionSequence`
      (:`then_0`
        (`self.Calculate Births For a City` _output_get))
      (:`then_1`
        (`self.ClearArrays` ; Clears Arrays that will contain moving scores
          (:`NewParam2`
            (bind _outactors_2 (`GameplayStatics.GetAllActorsOfClass` "/Game/Blueprints/City.City_C"))
            (for _array_element_2 _outactors_2
              (bind _output_get_2 (set `self.CityToMove` _array_element_2))
              (`KismetArrayLibrary.Array_Add` (`self.MovingScores`) (/ (`KismetMathLibrary.Conv_IntToDouble` (`/Game/Blueprints/City.Population` _output_get_2)) (`KismetMathLibrary.Conv_IntToDouble` (`/Game/Blueprints/City.Population` _output_get)))))
            (`self.Standardize Array` (`self.MovingScores`))))))))

(fn `UserConstructionScript`)